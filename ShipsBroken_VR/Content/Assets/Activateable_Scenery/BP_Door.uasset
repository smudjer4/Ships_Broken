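; Activateable door Blueprint that alternates between open and closed each time its OpenCheck event fires.
; A FlipFlop calls Open or Close, which set the Door component's world height to the actor's Z plus or minus LiftAmount.
; The Lerp alpha is fixed at 1, so the door jumps instantly, and Close lands below the actor's origin.
; An unconnected rotation-based opening remains in Open and never runs.
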(event `OpenCheck`
  (`/Engine/EditorBlueprintResources/StandardMacros.FlipFlop`
    (:`A`
      (`self.Open`))
    (:`B`
      (`self.Close`))))

(fn `Close`
  (bind (_returnvalue_x _returnvalue_y _returnvalue_z) (`KismetMathLibrary.BreakVector` (`self.K2_GetActorLocation`)))
  (`SceneComponent.K2_SetWorldLocation` (`self.Door`) (`KismetMathLibrary.MakeVector` _returnvalue_x _returnvalue_y (`KismetMathLibrary.Lerp` _returnvalue_z (- _returnvalue_z (`self.Lift amount`)) 1.0)) false false))

(fn `Open`
  (bind (_returnvalue_x _returnvalue_y _returnvalue_z) (`KismetMathLibrary.BreakVector` (`self.K2_GetActorLocation`)))
  (`SceneComponent.K2_SetWorldLocation` (`self.Door`) (`KismetMathLibrary.MakeVector` _returnvalue_x _returnvalue_y (`KismetMathLibrary.Lerp` _returnvalue_z (+ _returnvalue_z (`self.Lift amount`)) 1.0)) false false))

(fn `UserConstructionScript`)